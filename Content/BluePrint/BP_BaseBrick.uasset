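; Base breakable brick that grants a random power-up or penalty to the tank linked to the ball that breaks it.
; BeginPlay randomizes Life and one of eight effects, and each BP_Ball hit stores that ball and decrements Life.
; Tick checks for zero Life, then applies the effect through the stored ball's tank links and destroys the brick.
; Effects alter damage, bullets, balls or silence either tank, and set the tank's SkillName.
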(event OnComponentHit(StaticMesh)
  (params (HitComponent :type Primitive%20Component%20Object%20Reference) (OtherActor :type Actor%20Object%20Reference) (OtherComp :type Primitive%20Component%20Object%20Reference) (NormalImpulse :type Vector :default "0, 0, 0") (Hit :type Hit%20Result%20Structure%20%28by%20ref%29))
  (bind _asbp_ball (Utilities|Casting|CastToBP_Ball OtherActor))
  (Variables|Default|SetBall _asbp_ball)
  (Variables|Default|Setlife (- (Variables|Default|Getlife) 1)))

(event Custom|isBroken
  (if (<= (Variables|Default|Getlife) 0)
    (CallFunction|ExecWepon)
    (Actor|DestroyActor)))

(event EventBeginPlay
  (CallFunction|InitAttribute))

(event Collision|EventActorBeginOverlap
  (params (OtherActor :type Actor%20Object%20Reference)))

(event EventTick
  (params (DeltaSeconds :type Float%20%28single-precision%29))
  (CallFunction|IsBroken))

(fn ConstructionScript)

(fn InitAttribute
  (Variables|Default|Setlife (Math|Random|RandomIntegerinRange 2 5))
  (CallFunction|RandomWepon))

(fn RandomWepon
  (bind _returnvalue (Math|Random|RandomInteger 8))
  (Variables|Default|Setwepon _returnvalue)
  (switch int _returnvalue))

(fn ExecWepon
  (bind _ball (Variables|Default|GetBall))
  (bind _balltanke (Variables|/Game/BluePrint/BP_Ball.BP_Ball_C|GetBallTanke _ball))
  (bind _tank (Variables|/Game/BluePrint/BP_BallTanke.BP_BallTanke_C|GetTank _balltanke))
  (switch int (Variables|Default|Getwepon)
    (:0
      (Default|DamageMulti _tank 1e+01 2.0)
      (Variables|/Game/BluePrint/BP_Tanke.BP_Tanke_C|SetskillName _tank "Damage*2"))
    (:1
      (Default|SilenceMulti (Variables|/Game/BluePrint/BP_Tanke.BP_Tanke_C|GetenemyTank _tank) 1e+01)
      (Variables|/Game/BluePrint/BP_Tanke.BP_Tanke_C|SetskillName _tank "Enemy Silence"))
    (:2
      (Default|DamageMulti _tank 1e+01 4.0)
      (Variables|/Game/BluePrint/BP_Tanke.BP_Tanke_C|SetskillName _tank "Damage*4"))
    (:3
      (Default|SilenceMulti _tank 5.0)
      (Variables|/Game/BluePrint/BP_Tanke.BP_Tanke_C|SetskillName _tank "Silence"))
    (:4
      (Default|MultiBullteNum _tank 4)
      (Variables|/Game/BluePrint/BP_Tanke.BP_Tanke_C|SetskillName _tank "Bullet count *4"))
    (:5
      (Default|AddBallNum _balltanke)
      (Variables|/Game/BluePrint/BP_Tanke.BP_Tanke_C|SetskillName _tank "Add ball"))
    (:6
      (Default|BallSpeedMulti _balltanke)
      (Variables|/Game/BluePrint/BP_Tanke.BP_Tanke_C|SetskillName _tank "Ball speed up"))
    (:7
      (Default|AddBullteNum _tank 50)
      (Variables|/Game/BluePrint/BP_Tanke.BP_Tanke_C|SetskillName _tank "Bullet count +50"))))
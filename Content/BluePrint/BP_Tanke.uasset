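; Auto-firing tank that sways and rotates on a sine wave, spawning BP_Bullets from an ammo count.
; Tick-driven Delays pace firing and ammo regeneration; larger ammo totals raise fire rate and bullet speed.
; Timed skills split or speed up its tracked bullets, clear the EnemyTank's, grant invincibility or spawn misty areas.
; Other events apply silence, damage or ammo multipliers, adopt bullets and accumulate damage taken; the death check is empty.
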(event Custom|OpenFire
  (bind _arrow (Variables|Default|GetArrow))
  (if (not (Variables|Default|GetsilenceStatu))
    (if (> (Variables|Default|GettotalNum) 0)
      (Utilities|FlowControl|Delay (Variables|Default|GetemitterSpeed))
      (bind _returnvalue (Game|SpawnActorfromClass "/Game/BluePrint/BP_Bullet.BP_Bullet_C" (Math|Transform|MakeTransform (Transformation|GetWorldLocation _arrow) (Transformation|GetWorldRotation _arrow) "0.150000,0.250000,0.150000") "Undefined" 0 0))
      (Variables|/Game/BluePrint/BP_Bullet.BP_Bullet_C|SettankResource _returnvalue self)
      (Variables|/Game/BluePrint/BP_Bullet.BP_Bullet_C|Setdamage _returnvalue (Variables|Default|Getdamage))
      (Utilities|Array|Add (Variables|Default|GetbulletArray) _returnvalue)
      (Variables|Default|SettotalNum (- (Variables|Default|GettotalNum) 1)))))

(event Custom|damageMulti
  (params (duration :type Float%20%28single-precision%29) (multi :type Float%20%28single-precision%29))
  (CallFunction|DamageDoubble (Math|Float|Truncate (* 5 multi)))
  (Utilities|FlowControl|Delay duration)
  (CallFunction|DamageDoubble 5))

(event Custom|removeAllBullet
  ;[1 1 1] 对应中级技能中 第1个
  (CallFunction|DestoryAllBullet (Variables|Default|GetenemyTank))
  (Variables|Default|SetskillName "Kill all bullet ")
  (Utilities|FlowControl|Delay 1e+01)
  (if (not (Utilities|Enum|NotEqual(Enum) (Variables|Default|GetskillName) "Kill all bullet "))
    (Variables|Default|SetskillName "None")))

(event Custom|mistyArea
  (for _index (range 0 5)
    (bind _returnvalue (Game|SpawnActorfromClass "/Game/BluePrint/BP_MistyArea.BP_MistyArea_C" (Math|Transform|MakeTransform (Math|Vector|MakeVector (Math|Random|RandomFloatinRange -2.5e+02 2.5e+02) (Math|Random|RandomFloatinRange -3e+02 3e+02) 5e+01) "0, 0, 0" "1,1,1") "Undefined" 0 0))
    (Variables|/Game/BluePrint/BP_MistyArea.BP_MistyArea_C|SettankTeam _returnvalue self)
    (Variables|Default|SetskillName "Misty area")
    (if (not (Utilities|Enum|NotEqual(Enum) (Variables|Default|GetskillName) "Misty area"))
      (Variables|Default|SetskillName "None"))))

(event Custom|invincibleStatu
  (Variables|Default|Setinvincible true)
  (Variables|Default|SetskillName "Invincible")
  (Utilities|FlowControl|Delay 1e+01)
  (Variables|Default|Setinvincible false)
  (if (not (Utilities|Enum|NotEqual(Enum) (Variables|Default|GetskillName) "Invincible"))
    (Variables|Default|SetskillName "None")))

(event Custom|destoryAllBullet
  (bind _bulletarray (Variables|Default|GetbulletArray))
  (bind _output_get (Variables|Default|SettmpBulletArray _bulletarray))
  (Utilities|Array|Clear _bulletarray)
  (for _array_element _output_get
    (Default|BulletDestory _array_element)))

(event Custom|bulletSpeedDouble
  (Utilities|FlowControl|Sequence
    (:then_0
      (for _array_element (Variables|Default|GetbulletArray)
        (Default|BulletSpeedDouble _array_element 2.5)))
    (:then_1
      (Variables|Default|SetemitterSpeed (/ (Variables|Default|GetemitterSpeed) 2.0))
      (Utilities|FlowControl|Delay 1e+01)
      (Variables|Default|SetemitterSpeed (* (Variables|Default|GetemitterSpeed) 2.0)))
    (:then_2
      (Variables|Default|SetskillName "Bullet speed double")
      (Utilities|FlowControl|Delay 1e+01)
      (if (not (Utilities|Enum|NotEqual(Enum) (Variables|Default|GetskillName) "Bullet speed double"))
        (Variables|Default|SetskillName "None")))))

(event Custom|silenceMulti
  (params (duration :type Float%20%28single-precision%29))
  (Variables|Default|SetsilenceStatu true)
  (Utilities|FlowControl|Delay duration)
  (Variables|Default|SetsilenceStatu false))

(event Custom|damageInjured
  (params (damage :type Integer))
  (if (not (Variables|Default|Getinvincible))
    (Variables|Default|SettotalDamage (+ (Variables|Default|GettotalDamage) damage))))

(event Custom|installBullet
  (params (bullet :type BP%20Bullet%20Object%20Reference))
  (if (Utilities|IsValid bullet)
    (Variables|/Game/BluePrint/BP_Bullet.BP_Bullet_C|Setdamage bullet (Variables|Default|Getdamage))
    (Utilities|Array|Add (Variables|Default|GetbulletArray) bullet)
    (Variables|/Game/BluePrint/BP_Bullet.BP_Bullet_C|SettankResource bullet self)))

(event Custom|addBullteNum
  (params (addNum :type Integer))
  (Variables|Default|SettotalNum (+ (Variables|Default|GettotalNum) addNum)))

(event Custom|multiBullteNum
  (params (multi :type Integer))
  (Variables|Default|SettotalNum (* (Variables|Default|GettotalNum) multi)))

(event Custom|bulletSplite
  (bind _bulletarray (Variables|Default|GetbulletArray))
  (bind _output_get (Variables|Default|SettmpBulletArray _bulletarray))
  (Utilities|Array|Clear _bulletarray)
  (Variables|Default|SetskillName "Bullet Splite")
  (for _array_element _output_get
    (Default|BulletSplit _array_element)
    (Actor|DestroyActor _array_element))
  (Utilities|FlowControl|Delay 1e+01)
  (if (not (Utilities|Enum|NotEqual(Enum) (Variables|Default|GetskillName) "Bullet Splite"))
    (Variables|Default|SetskillName "None")))

(event EventBeginPlay
  (Utilities|Array|Clear (Variables|Default|GettmpBulletArray))
  (Utilities|Array|Clear (Variables|Default|GetbulletArray)))

(event EventTick
  (params (DeltaSeconds :type Float%20%28single-precision%29))
  (CallFunction|TAutoRotation DeltaSeconds)
  (CallFunction|OpenFire)
  (CallFunction|UpdateBulletEmitterSpeed)
  (Utilities|FlowControl|Delay 1.0)
  (CallFunction|AddBullteNum 2))

(fn ConstructionScript)

(fn TAutoRotation
  (params (deltaSeconds :type Float%20%28single-precision%29))
  (bind _pt (Variables|Default|Getpt))
  (bind _output_get (Variables|Default|SettotalFrame (+ (Variables|Default|GettotalFrame) deltaSeconds)))
  (Transformation|SetRelativeRotation _pt (Math|Rotator|MakeRotator 9e+01 0.0 (* 30 (Math|Trig|Sin(Radians) (* _output_get 0.5)))) false false)
  (Transformation|SetRelativeLocation _pt (Math|Vector|MakeVector (* 250 (Math|Trig|Sin(Radians) (* _output_get 0.5))) 0.0 0.0) false false))

(fn TIsDead)

(fn DamageDoubble
  (params (multi :type Integer))
  (for _array_element (Variables|Default|GetbulletArray)
    (Variables|/Game/BluePrint/BP_Bullet.BP_Bullet_C|Setdamage _array_element multi)))

(fn UpdateBulletEmitterSpeed
  (bind _totalnum (Variables|Default|GettotalNum))
  (bind _returnvalue (Math|Conversions|ToFloat(Integer) _totalnum))
  (Variables|Default|SetemitterSpeed (Math|Float|MapRangeClamped _returnvalue 1e+02 5e+03 0.3 0.1))
  (for _array_element (Variables|Default|GetbulletArray)
    (Default|BulletSpeedDouble _array_element (Math|Float|MapRangeClamped _returnvalue 1e+02 5e+03 1.0 2.5))))
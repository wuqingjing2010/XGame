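; Status display Blueprint that shows a tank's stats in the world through a TextRender component.
; ShowMessage builds one string from the referenced tank's display name, total damage, bullet count, skill name (labelled as buffer) and ball array length, then sets it as the text.
; It runs from the construction script and again every Tick, polling the values rather than reacting to changes.
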(event EventBeginPlay)

(event Collision|EventActorBeginOverlap
  (params (OtherActor :type Actor%20Object%20Reference)))

(event EventTick
  (params (DeltaSeconds :type Float%20%28single-precision%29))
  (CallFunction|ShowMessage))

(fn ConstructionScript
  (CallFunction|ShowMessage))

(fn ShowMessage
  (bind _tank (Variables|Default|GetTank))
  (bind _tank_2 (Variables|/Game/BluePrint/BP_BallTanke.BP_BallTanke_C|GetTank _tank))
  (Rendering|Components|TextRender|SetText (Variables|Default|GetTextRender) (Utilities|Text|ToText(String) (Utilities|String|Append (Utilities|String|Append (Utilities|GetDisplayName _tank_2) " 
TotalDamage:") (Utilities|String|ToString(Integer) (Variables|/Game/BluePrint/BP_Tanke.BP_Tanke_C|GettotalDamage _tank_2)) " 
BulletNum:" (Utilities|String|ToString(Integer) (Variables|/Game/BluePrint/BP_Tanke.BP_Tanke_C|GettotalNum _tank_2)) " 
Buffer:" (Variables|/Game/BluePrint/BP_Tanke.BP_Tanke_C|GetskillName _tank_2) " 
BallNum:" (Utilities|String|ToString(Integer) (Utilities|Array|Length (Variables|/Game/BluePrint/BP_BallTanke.BP_BallTanke_C|GetBallArray _tank)))))))
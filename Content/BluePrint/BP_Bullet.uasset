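; Tank projectile Blueprint that damages the enemy tank recorded in TankResource and destroys itself on impact.
; Box hit events destroy both bullets when two collide, and matching the enemy tank relies on class and display name.
; bulletSplit spawns a row of twelve bullets registered with TankResource, whose array drops each on destruction.
; bulletSpeedDouble rescales physics velocity by a multiplier, then after ten seconds applies its inverse to base speed.
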(event OnComponentHit(Box)
  (params (HitComponent :type Primitive%20Component%20Object%20Reference) (OtherActor :type Actor%20Object%20Reference) (OtherComp :type Primitive%20Component%20Object%20Reference) (NormalImpulse :type Vector :default "0, 0, 0") (Hit :type Hit%20Result%20Structure%20%28by%20ref%29))
  (bind _returnvalue (Utilities|GetClass OtherActor))
  (bind _tankresource (Variables|Default|GettankResource))
  (bind _enemytank (Variables|/Game/BluePrint/BP_Tanke.BP_Tanke_C|GetenemyTank _tankresource))
  (Utilities|FlowControl|Sequence
    (:then_0
      (if (== _returnvalue "BP_Bullet_C")
        (bind _asbp_bullet (Utilities|Casting|CastToBP_Bullet OtherActor))
        (CallFunction|BulletDestory _asbp_bullet)
        (CallFunction|BulletDestory)))
    (:then_2
      (if (and (== _returnvalue "/Game/BluePrint/BP_Tanke.BP_Tanke_C") (Utilities|Enum|Equal(Enum) (Utilities|GetDisplayName OtherActor) (Utilities|GetDisplayName _enemytank)))
        (Default|DamageInjured _enemytank (Variables|Default|Getdamage))
        (CallFunction|BulletDestory)
        (else
          (CallFunction|BulletDestory))))))

(event Custom|bulletDestory
  (Utilities|Array|RemoveItem (Variables|/Game/BluePrint/BP_Tanke.BP_Tanke_C|GetbulletArray (Variables|Default|GettankResource)) self)
  (Actor|DestroyActor))

(event Custom|bulletSplit
  (bind _self self)
  (bind _returnvalue (Transformation|GetActorTransform _self))
  (for _index (range 0 11)
    (bind _returnvalue_2 (Game|SpawnActorfromClass "BP_Bullet_C" (Math|Transform|MakeTransform (+ (- (.location _returnvalue) "160.000000,-20.000000, 0") (* "20.000000, 0, 0" _index)) (.rotation _returnvalue) (.scale _returnvalue)) "AlwaysSpawn" 0 0))
    (Default|InstallBullet (Variables|Default|GettankResource) _returnvalue_2)))

(event Custom|bulletSpeedDouble
  (params (speedMult :type Float%20%28single-precision%29))
  (bind _box (Variables|Default|GetBox))
  (bind _returnvalue (Physics|GetPhysicsLinearVelocity _box "None"))
  (Physics|SetPhysicsLinearVelocity _box (* (* (Math|Vector|Normalize _returnvalue) 2e+02) speedMult) false "None")
  (Utilities|FlowControl|Delay 1e+01)
  (Physics|SetPhysicsLinearVelocity _box (* (* (Math|Vector|Normalize _returnvalue) 2e+02) (/ 1.0 speedMult)) false "None"))

(fn ConstructionScript)
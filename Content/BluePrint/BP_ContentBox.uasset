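; BP_ContentBox is an actor that configures a Niagara system as a grid, apparently of meshes, from count, size and start-position variables.
; The construction script derives dimensions from counts, cell size, padding and a distance divisor, then passes them with offset, X/Y counts and mesh scale to Niagara user parameters.
; The event graph, changeColor event and both functions, T_currentResult and getAllBullet, are empty stubs.
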(event Custom|changeColor)

(event EventBeginPlay)

(event Collision|EventActorBeginOverlap
  (params (OtherActor :type Actor%20Object%20Reference)))

(event EventTick
  (params (DeltaSeconds :type Float%20%28single-precision%29)))

(fn ConstructionScript
  (bind _niagara (Variables|Default|GetNiagara))
  (Class|NiagaraComponent|SetNiagaraVariableVec3 _niagara "User.XYZDimensions" (/ (Math|Vector|MakeVector (Math|Conversions|ToFloat(Integer) (+ (* (Variables|Size|GetwidthCount) (Variables|Size|Getsize)) (Variables|Default|Getescap))) (Math|Conversions|ToFloat(Integer) (+ (* (Variables|Size|GetlegthCount) (Variables|Size|Getsize)) (Variables|Default|Getescap))) 1e+01) (Variables|Size|Getdistance)))
  (Class|NiagaraComponent|SetNiagaraVariableVec3 _niagara "User.offset" (Math|Vector|MakeVector (Math|Conversions|ToFloat(Integer) (Variables|Size|GetstartX)) (Math|Conversions|ToFloat(Integer) (Variables|Size|GetstartY)) 0.0))
  (Class|NiagaraComponent|SetNiagaraVariableInt _niagara "User.XCount" (Variables|Size|GetwidthCount))
  (Class|NiagaraComponent|SetNiagaraVariableInt _niagara "User.YCount" (Variables|Size|GetlegthCount))
  (Niagara|SetNiagaraVariable(Float) _niagara "User.MeshScale" (/ (Math|Conversions|ToFloat(Integer) (Variables|Size|Getsize)) 1e+02)))

(fn TCurrentResult)

(fn GetAllBullet)
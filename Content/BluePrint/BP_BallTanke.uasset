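; BP_BallTanke is a ball launcher that spawns BP_Ball actors at its arrow from a limited ball count, starting at BeginPlay.
; Each ball gets a fixed +Y velocity plus part of the Cube's sampled movement, and a back-reference to the launcher.
; Delay-throttled Tick checks watch the tracked ball array, adding and firing a ball after a wait when it is empty.
; Events also add balls or speed up all tracked ones.
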(event Custom|emitterBall
  (if (> (Variables|Default|GetballNum) 0)
    (CallFunction|EmitterBallFunction)))

(event Custom|ballSpeedMulti
  (for _array_element (Variables|Default|GetBallArray)
    (Default|BallSpeedDouble _array_element 1.5)))

(event Custom|addBallNum
  (Variables|Default|SetballNum (+ (Variables|Default|GetballNum) 1)))

(event EventBeginPlay
  (Variables|Default|SetlastPostion (Transformation|GetWorldLocation (Variables|Default|GetCube)))
  (CallFunction|EmitterBall))

(event EventTick
  (params (DeltaSeconds :type Float%20%28single-precision%29))
  (Utilities|FlowControl|Sequence
    (:then_0
      (Variables|Default|Setvelocity (- (Transformation|GetWorldLocation (Variables|Default|GetCube)) (Variables|Default|GetlastPostion)))
      (Utilities|FlowControl|Delay 0.5)
      (Variables|Default|SetlastPostion (Transformation|GetWorldLocation (Variables|Default|GetCube))))
    (:then_1
      (Utilities|FlowControl|Delay 0.2)
      (CallFunction|CheckBallExists))
    (:then_2
      (if (not (Variables|Default|GetballExists))
        (Utilities|FlowControl|Delay 5.0)
        (Variables|Default|SetballNum (+ (Variables|Default|GetballNum) 1))
        (CallFunction|EmitterBall)))))

(fn ConstructionScript)

(fn EmitterBallFunction
  (bind _arrow (Variables|Default|GetArrow))
  (bind _returnvalue (Game|SpawnActorfromClass "/Game/BluePrint/BP_Ball.BP_Ball_C" (Math|Transform|MakeTransform (Transformation|GetWorldLocation _arrow) (Transformation|GetWorldRotation _arrow) "0.400000,0.400000,0.400000") "Undefined" 0 0))
  (Physics|SetPhysicsLinearVelocity (Variables|/Game/BluePrint/BP_Ball.BP_Ball_C|GetBouncSphere _returnvalue) (+ (* (Variables|Default|Getvelocity) 0.2) "0.000000,500.000000, 0") false "None")
  (Variables|/Game/BluePrint/BP_Ball.BP_Ball_C|SetBallTanke _returnvalue self)
  (Variables|Default|SetballNum (- (Variables|Default|GetballNum) 1))
  (Utilities|Array|Add (Variables|Default|GetBallArray) _returnvalue))

(fn CheckBallExists
  (Variables|Default|SetballExists (> (Utilities|Array|Length (Variables|Default|GetBallArray)) 0))
  (return))
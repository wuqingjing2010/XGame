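; BP_MidBrick is a breakable brick that grants a random tank effect when destroyed by balls.
; On spawn it rolls random hit points and one of five effects: bullet split, bullet removal, double speed, misty area or invincibility.
; Each BP_Ball hit costs one life and stores that ball.
; A per-tick check applies the effect to the last ball's tank at zero life, then destroys the brick.
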(event OnComponentHit(StaticMesh)
  (params (HitComponent :type Primitive%20Component%20Object%20Reference) (OtherActor :type Actor%20Object%20Reference) (OtherComp :type Primitive%20Component%20Object%20Reference) (NormalImpulse :type Vector :default "0, 0, 0") (Hit :type Hit%20Result%20Structure%20%28by%20ref%29))
  (bind _asbp_ball (Utilities|Casting|CastToBP_Ball OtherActor))
  (Variables|Default|SetBall _asbp_ball)
  (Variables|Default|Setlife (- (Variables|Default|Getlife) 1)))

(event Custom|isBroken
  (if (<= (Variables|Default|Getlife) 0)
    (CallFunction|ExecWepon)
    (Actor|DestroyActor)))

(event EventBeginPlay
  (CallFunction|InitAttribute))

(event Collision|EventActorBeginOverlap
  (params (OtherActor :type Actor%20Object%20Reference)))

(event EventTick
  (params (DeltaSeconds :type Float%20%28single-precision%29))
  (CallFunction|IsBroken))

(fn ConstructionScript)

(fn InitAttribute
  (Variables|Default|Setlife (Math|Random|RandomIntegerinRange 15 20))
  (CallFunction|RandomWepon))

(fn RandomWepon
  (Variables|Default|Setwepon (Math|Random|RandomInteger 5)))

(fn ExecWepon
  (bind _ball (Variables|Default|GetBall))
  (bind _balltanke (Variables|/Game/BluePrint/BP_Ball.BP_Ball_C|GetBallTanke _ball))
  (bind _tank (Variables|/Game/BluePrint/BP_BallTanke.BP_BallTanke_C|GetTank _balltanke))
  (switch int (Variables|Default|Getwepon)
    (:0
      (Default|BulletSplite _tank))
    (:1
      (Default|RemoveAllBullet _tank))
    (:2
      (Default|BulletSpeedDouble _tank))
    (:3
      (Default|MistyArea _tank))
    (:4
      (Default|InvincibleStatu _tank))))
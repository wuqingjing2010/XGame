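; Physics ball owned by a BP_BallTanke: hitting that tank adds to its total, while hitting another tank transfers ownership to it.
; Each tick applies a logarithmic force that steers speed toward a target, then checks bounds and speed.
; Leaving the Y bounds destroys the ball and lowers the owner's BallNum; nearly stopping destroys it and raises BallNum.
; A speed event multiplies velocity, then divides it back after a delay.
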(event OnComponentHit(BouncSphere)
  (params (HitComponent :type Primitive%20Component%20Object%20Reference) (OtherActor :type Actor%20Object%20Reference) (OtherComp :type Primitive%20Component%20Object%20Reference) (NormalImpulse :type Vector :default "0, 0, 0") (Hit :type Hit%20Result%20Structure%20%28by%20ref%29))
  (bind _self self)
  (if (== (Utilities|GetClass OtherActor) "/Game/BluePrint/BP_BallTanke.BP_BallTanke_C")
    (if (== OtherActor (Variables|Default|GetBallTanke))
      (Variables|/Game/BluePrint/BP_Tanke.BP_Tanke_C|SettotalNum (Variables|/Game/BluePrint/BP_BallTanke.BP_BallTanke_C|GetTank (Variables|Default|GetBallTanke)) (+ (Variables|/Game/BluePrint/BP_Tanke.BP_Tanke_C|GettotalNum (Variables|/Game/BluePrint/BP_BallTanke.BP_BallTanke_C|GetTank (Variables|Default|GetBallTanke))) 10))
      (else
        (bind _asbp_ball_tanke (Utilities|Casting|CastToBP_BallTanke OtherActor))
        (Utilities|Array|RemoveItem (Variables|/Game/BluePrint/BP_BallTanke.BP_BallTanke_C|GetBallArray (Variables|Default|GetBallTanke)) _self)
        (Utilities|Array|Add (Variables|/Game/BluePrint/BP_BallTanke.BP_BallTanke_C|GetBallArray _asbp_ball_tanke) _self)
        (Variables|Default|SetBallTanke _asbp_ball_tanke)))))

(event Custom|isOut
  (bind _self self)
  (bind _balltanke (Variables|Default|GetBallTanke))
  (bind _bouncsphere (Variables|Default|GetBouncSphere _self))
  (bind _returnvalue (Transformation|GetWorldLocation _bouncsphere))
  (if (or (<= (.y _returnvalue) -6.8e+02) (>= (.y _returnvalue) 6.8e+02))
    (Utilities|Array|RemoveItem (Variables|/Game/BluePrint/BP_BallTanke.BP_BallTanke_C|GetBallArray _balltanke) self)
    (Actor|DestroyActor)
    (Variables|/Game/BluePrint/BP_BallTanke.BP_BallTanke_C|SetballNum _balltanke (- (Variables|/Game/BluePrint/BP_BallTanke.BP_BallTanke_C|GetballNum _balltanke) 1))))

(event Custom|ballSpeedDouble
  (params (speed :type Float%20%28single-precision%29))
  (CallFunction|SpeedDouble speed)
  (Utilities|FlowControl|Delay 1e+01)
  (CallFunction|SpeedDouble (/ 1.0 speed)))

(event EventBeginPlay)

(event Collision|EventActorBeginOverlap
  (params (OtherActor :type Actor%20Object%20Reference)))

(event EventTick
  (params (DeltaSeconds :type Float%20%28single-precision%29))
  (CallFunction|AddForce)
  (CallFunction|IsOut)
  (CallFunction|CheckBallSpeed))

(fn ConstructionScript)

(fn SpeedDouble
  (params (multi :type Float%20%28single-precision%29))
  (bind _bouncsphere (Variables|Default|GetBouncSphere))
  (bind _returnvalue (Physics|GetPhysicsLinearVelocity _bouncsphere "None"))
  (Physics|SetPhysicsLinearVelocity _bouncsphere (* _returnvalue multi) false "None"))

(fn AddForce
  (bind _self self)
  (bind _bouncsphere (Variables|Default|GetBouncSphere _self))
  (if (Utilities|IsValid _bouncsphere)
    (bind _returnvalue (Physics|GetPhysicsLinearVelocity _bouncsphere "None"))
    (Physics|AddForce _bouncsphere (* (* (* (Math|Vector|Normalize _returnvalue) (Physics|GetMass _bouncsphere)) 1.0) (Math|Float|Loge (/ 5e+02 (Math|Vector|VectorLength _returnvalue)))) "None" false)))

(fn CheckBallSpeed
  (bind _balltanke (Variables|Default|GetBallTanke))
  (bind _bouncsphere (Variables|Default|GetBouncSphere))
  (if (Utilities|IsValid _bouncsphere)
    (bind _returnvalue (Physics|GetPhysicsLinearVelocity _bouncsphere "None"))
    (if (<= (Math|Vector|VectorLength _returnvalue) 2.0)
      (Variables|/Game/BluePrint/BP_BallTanke.BP_BallTanke_C|SetballNum _balltanke (+ (Variables|/Game/BluePrint/BP_BallTanke.BP_BallTanke_C|GetballNum _balltanke) 1))
      (Utilities|Array|RemoveItem (Variables|/Game/BluePrint/BP_BallTanke.BP_BallTanke_C|GetBallArray _balltanke) self)
      (Actor|DestroyActor))))